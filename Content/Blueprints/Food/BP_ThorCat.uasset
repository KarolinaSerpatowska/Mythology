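; BP_ThorCat is the possessable cat character for a color-based minigame, hidden until a player controls it.
; On restart under player control it shows itself and the HUD, then after a delay starts the color widget at the GameInstance's drink speed and switches the cat's animation.
; Interact and Pause drive the color widget.
; When the minigame ends, it hides, returns possession to BP_FoodPlayer and flags CatDone on the GameInstance.
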(event Custom|EndThis
  (bind _returnvalue (Game|GetPlayerController 0))
  (bind _returnvalue_2 (Actor|GetActorOfClass "/Game/Blueprints/Food/BP_FoodPlayer.BP_FoodPlayer_C"))
  (Widget|SetVisibility (Variables|Default|GetUIMinigame) "Hidden")
  (Rendering|SetActorHiddenInGame true)
  (Pawn|Possess _returnvalue _returnvalue_2)
  (bind _asbp_my_player_controller (Utilities|Casting|CastToBP_MyPlayerController _returnvalue))
  (Class|MyPlayerController|ChangePawn _asbp_my_player_controller)
  (bind _asbp_game_instance (Utilities|Casting|CastToBP_GameInstance (Game|GetGameInstance)))
  (Variables|/Game/Blueprints/BP_GameInstance.BP_GameInstance_C|SetCatDone _asbp_game_instance true))

(event EventBeginPlay
  (Rendering|SetActorHiddenInGame true))

(event EventPause
  (bind _uiminigame (Variables|Default|GetUIMinigame))
  (bind _ui_colorwidget (Variables|/Game/UI/UI_Minigame.UI_Minigame_C|GetUI_ColorWidget _uiminigame))
  (if (and (Variables|/Game/UI/UI_ColorWidget.UI_ColorWidget_C|GetIsPaused _ui_colorwidget) (Class|UserWidget|IsPlayingAnimation _ui_colorwidget))
    (Default|UnpauseAnim _ui_colorwidget (Variables|Default|GetMinigame%20Drink%20Speed))
    (else
      (Default|PauseAnim _ui_colorwidget))))

(event EventInteract
  (bind _uiminigame (Variables|Default|GetUIMinigame))
  (bind _ui_colorwidget (Variables|/Game/UI/UI_Minigame.UI_Minigame_C|GetUI_ColorWidget _uiminigame))
  (if (Class|UserWidget|IsPlayingAnimation _ui_colorwidget)
    (Default|PauseColor _ui_colorwidget)
    (Default|StartColor _ui_colorwidget (Variables|Default|GetMinigame%20Drink%20Speed))))

(event EventRestarted
  (if (Pawn|IsPlayerControlled)
    (bind _hudwidgetinstance (Variables|Default|GetHUDWidgetInstance)
      (:then
        (Widget|SetVisibility _hudwidgetinstance "Visible")
        (bind _asui_minigame (Utilities|Casting|CastToUI_Minigame _hudwidgetinstance))
        (bind _output_get (Variables|Default|SetUIMinigame _asui_minigame))
        (Rendering|SetActorHiddenInGame false)
        (Utilities|FlowControl|Delay 3.0)
        (bind _asbp_game_instance (Utilities|Casting|CastToBP_GameInstance (Game|GetGameInstance)))
        (bind _output_get_2 (Variables|Default|SetMinigame%20Drink%20Speed (Variables|/Game/Blueprints/BP_GameInstance.BP_GameInstance_C|GetMinigameDrinkSpeed _asbp_game_instance)))
        (Default|StartColor (Variables|/Game/UI/UI_Minigame.UI_Minigame_C|GetUI_ColorWidget _output_get) _output_get_2)
        (EventDispatchers|BindEventtoEndMinigame (Variables|/Game/UI/UI_Minigame.UI_Minigame_C|GetUI_ColorWidget _output_get) (delegate Custom|EndThis))
        (bind _asabp_cat (Utilities|Casting|CastToABP_Cat (Components|SkeletalMesh|GetAnimInstance (Variables|Character|GetMesh))))
        (Variables|/Game/Meshes/Characters/Cat/ABP_Cat.ABP_Cat_C|SetChangeAnim _asabp_cat true))
      (:else))))

(fn ConstructionScript)