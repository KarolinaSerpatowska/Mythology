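; Behavior tree task, apparently used in dialogue, that starts the food minigame.
; It copies the food minigame duration from BP_GameInstance to the BP_FoodPlayer found in the level and starts that actor's minigame.
; It then spawns a BP_Pickup at every BP_FoodSpawner's transform and immediately finishes successfully, without waiting for the minigame to end.
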(event EventReceiveExecuteAI
  (params (OwnerController :type AI%20Controller%20Object%20Reference) (ControlledPawn :type Pawn%20Object%20Reference))
  (bind _asbp_game_instance (Utilities|Casting|CastToBP_GameInstance (Game|GetGameInstance)))
  (bind _returnvalue (Actor|GetActorOfClass "/Game/Blueprints/Food/BP_FoodPlayer.BP_FoodPlayer_C"))
  (Variables|/Script/MythologyCPP.FoodPlayer|Setseconds _returnvalue (Variables|/Game/Blueprints/BP_GameInstance.BP_GameInstance_C|GetMinigameFoodSec _asbp_game_instance))
  (Class|FoodPlayer|StartFoodMinigame _returnvalue)
  (bind _outactors (Actor|GetAllActorsOfClass "/Game/Blueprints/Food/BP_FoodSpawner.BP_FoodSpawner_C"))
  (for _array_element _outactors
    (Game|SpawnActorfromClass "/Game/Blueprints/BP_Pickup.BP_Pickup_C" (Transformation|GetActorTransform _array_element) "Undefined" "MultiplyWithRoot" 0 0))
  (AI|BehaviorTree|FinishExecute true))