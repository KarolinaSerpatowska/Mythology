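; ReplyTask is a Behavior Tree task that presents dialogue reply options to the player and records the chosen one.
; On execute it gets the dialogue widget from the blackboard, binds to its OnReplyFinished event and passes it the reply texts.
; When a reply finishes, it unbinds, writes the reply index to a blackboard key and finishes successfully, so the task stays latent until then.
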(event Custom|OnReplyFinished_Event
  (params (ReplyIndex :type Integer))
  (EventDispatchers|UnbindEventfromOnReplyFinished (.AsUI%20Dialogue%20Widget (Utilities|Casting|CastToUI_DialogueWidget (Class|BTFunctionLibrary|GetBlackboardValueasObject (Variables|Default|GetDialogueWidget)))) (delegate Custom|OnReplyFinished_Event))
  (Class|BTFunctionLibrary|SetBlackboardValueasInt (Variables|Default|GetOutReplyIndex) ReplyIndex)
  (AI|BehaviorTree|FinishExecute true))

(event EventReceiveExecuteAI
  (params (OwnerController :type AI%20Controller%20Object%20Reference) (ControlledPawn :type Pawn%20Object%20Reference))
  (bind _dialoguewidget (Variables|Default|GetDialogueWidget))
  (bind _returnvalue (Class|BTFunctionLibrary|GetBlackboardValueasObject _dialoguewidget))
  (bind _asui_dialogue_widget (Utilities|Casting|CastToUI_DialogueWidget _returnvalue))
  (EventDispatchers|AssignOnReplyFinished _asui_dialogue_widget (delegate Custom|OnReplyFinished_Event))
  (Default|Reply _asui_dialogue_widget (Variables|Default|GetRepliesText)))