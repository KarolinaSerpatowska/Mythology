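; A behavior tree task in the dialogue tasks folder that restores quest progress from BP_GameInstance into the blackboard.
; On execute it copies the race, drink, cat, food and fight flags into blackboard keys, then finishes successfully.
; If Utgard has been opened before, it also sets that flag and marks the first sequence and first Skyrmir step as done.
; A failed game instance cast stops it without finishing.
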(event EventReceiveExecuteAI
  (params (OwnerController :type AI%20Controller%20Object%20Reference) (ControlledPawn :type Pawn%20Object%20Reference))
  (bind _asbp_game_instance (Utilities|Casting|CastToBP_GameInstance (Game|GetGameInstance)))
  (if (Variables|/Game/Blueprints/BP_GameInstance.BP_GameInstance_C|GetUtgardFirstOpened _asbp_game_instance)
    (Class|BTFunctionLibrary|SetBlackboardValueasBool (Variables|Default|GetUtgardFirstOpened) (Variables|/Game/Blueprints/BP_GameInstance.BP_GameInstance_C|GetUtgardFirstOpened _asbp_game_instance))
    (Class|BTFunctionLibrary|SetBlackboardValueasBool (Variables|Default|GetRaceSet) (Variables|/Game/Blueprints/BP_GameInstance.BP_GameInstance_C|GetRaceDone _asbp_game_instance))
    (Class|BTFunctionLibrary|SetBlackboardValueasBool (Variables|Default|GetFirstSeqDone) true)
    (Class|BTFunctionLibrary|SetBlackboardValueasBool (Variables|Default|GetSkyrmirFirstDone) true)
    (Class|BTFunctionLibrary|SetBlackboardValueasBool (Variables|Default|GetDrinkSet) (Variables|/Game/Blueprints/BP_GameInstance.BP_GameInstance_C|GetDrinkDone _asbp_game_instance))
    (Class|BTFunctionLibrary|SetBlackboardValueasBool (Variables|Default|GetCatSet) (Variables|/Game/Blueprints/BP_GameInstance.BP_GameInstance_C|GetCatDone _asbp_game_instance))
    (Class|BTFunctionLibrary|SetBlackboardValueasBool (Variables|Default|GetFoodStart) (Variables|/Game/Blueprints/BP_GameInstance.BP_GameInstance_C|GetFoodStart _asbp_game_instance))
    (Class|BTFunctionLibrary|SetBlackboardValueasBool (Variables|Default|GetFoodSet) (Variables|/Game/Blueprints/BP_GameInstance.BP_GameInstance_C|GetFoodDone _asbp_game_instance))
    (Class|BTFunctionLibrary|SetBlackboardValueasBool (Variables|Default|GetFistsDone) (Variables|/Game/Blueprints/BP_GameInstance.BP_GameInstance_C|GetFightDone _asbp_game_instance))
    (else
      (Class|BTFunctionLibrary|SetBlackboardValueasBool (Variables|Default|GetRaceSet) (Variables|/Game/Blueprints/BP_GameInstance.BP_GameInstance_C|GetRaceDone _asbp_game_instance))
      (Class|BTFunctionLibrary|SetBlackboardValueasBool (Variables|Default|GetDrinkSet) (Variables|/Game/Blueprints/BP_GameInstance.BP_GameInstance_C|GetDrinkDone _asbp_game_instance))
      (Class|BTFunctionLibrary|SetBlackboardValueasBool (Variables|Default|GetCatSet) (Variables|/Game/Blueprints/BP_GameInstance.BP_GameInstance_C|GetCatDone _asbp_game_instance))
      (Class|BTFunctionLibrary|SetBlackboardValueasBool (Variables|Default|GetFoodStart) (Variables|/Game/Blueprints/BP_GameInstance.BP_GameInstance_C|GetFoodStart _asbp_game_instance))
      (Class|BTFunctionLibrary|SetBlackboardValueasBool (Variables|Default|GetFoodSet) (Variables|/Game/Blueprints/BP_GameInstance.BP_GameInstance_C|GetFoodDone _asbp_game_instance))
      (Class|BTFunctionLibrary|SetBlackboardValueasBool (Variables|Default|GetFistsDone) (Variables|/Game/Blueprints/BP_GameInstance.BP_GameInstance_C|GetFightDone _asbp_game_instance))))
  (AI|BehaviorTree|FinishExecute true))