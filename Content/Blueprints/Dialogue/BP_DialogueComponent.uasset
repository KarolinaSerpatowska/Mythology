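; Dialogue component that runs a behavior-tree-driven conversation when a player interacts with it.
; On BeginPlay it spawns its own AI controller to act as the dialogue tree runner.
; Interaction, gated by CanInteract, opens the dialogue widget with UI-only input, starts the tree and passes the widget through the blackboard.
; The widget's exit event stops the tree, removes the widget and restores game input.
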(event Custom|OnExit
  (bind _playercontroller (Variables|Default|GetPlayerController))
  (Input|SetInputModeGameOnly _playercontroller false)
  (Variables|/Script/Engine.PlayerController|SetbShowMouseCursor _playercontroller false)
  (AI|Logic|StopLogic (Variables|/Script/AIModule.AIController|GetBrainComponent (Variables|Default|GetAIController)) "")
  (Widget|RemovefromParent (Variables|Default|GetDialogueWidget)))

(event EventBeginPlay
  (bind _returnvalue (Game|SpawnActorfromClass "/Script/MythologyCPP.MyAIController" (Math|Transform|MakeTransform "0, 0, 0") "Undefined" "MultiplyWithRoot" 0 0))
  (Variables|Default|SetAiController _returnvalue))

(event EventOnInteraction
  (params (player :type Character%20Object%20Reference))
  (bind _aicontroller (Variables|Default|GetAIController))
  (if (Variables|Default|GetCanInteract)
    (bind _asmy_player_controller (Utilities|Casting|CastToMyPlayerController (Pawn|GetController player)))
    (Variables|Default|SetPlayerController _asmy_player_controller)
    (bind _returnvalue (UserInterface|CreateWidget "/Game/UI/UI_DialogueWidget.UI_DialogueWidget_C" _asmy_player_controller))
    (bind _output_get (Variables|Default|SetDialogueWidget _returnvalue))
    (if (not (UserInterface|Viewport|IsinViewport _output_get))
      (UserInterface|Viewport|AddtoViewport (Variables|Default|GetDialogueWidget) 0)
      (Input|SetInputModeUIOnly (Variables|Default|GetPlayerController) (Variables|Default|GetDialogueWidget) "DoNotLock" false)
      (Variables|/Script/Engine.PlayerController|SetbShowMouseCursor (Variables|Default|GetPlayerController) true)
      (EventDispatchers|BindEventtoOnExit (Variables|Default|GetDialogueWidget) (delegate Custom|OnExit))
      (AI|RunBehaviorTree _aicontroller (Variables|Default|GetDialogueTree))
      (bind _blackboardcomponent (Class|AIController|UseBlackboard _aicontroller (Variables|Default|GetBlackboard%20Asset)))
      (AI|Components|Blackboard|SetValueasObject _blackboardcomponent (Utilities|Name|MakeLiteralName "DialogueWidget") (Variables|Default|GetDialogueWidget)))))